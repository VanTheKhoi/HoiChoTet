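; BP_MovementComponent is an actor component that turns player driving input into vehicle movement.
; On BeginPlay it casts its owner to WheeledVehiclePawn and caches that pawn's VehicleMovementComponent.
; Enhanced Input actions for throttle, brake and steer pass their value straight to that component on both Triggered and Completed.
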(event Input|EnhancedActionEvents|EnhancedInputActionIA_Vehicle_Steer
  (params (ActionValue :type Float%20%28double-precision%29) (ElapsedSeconds :type Float%20%28double-precision%29) (TriggeredSeconds :type Float%20%28double-precision%29) (InputAction :type Input%20Action%20Object%20Reference :default "/Game/VehicleConfigurator/Core/Inputs/IA_Vehicle_Steer.IA_Vehicle_Steer"))
  (:Triggered
    (Class|ChaosVehicleMovementComponent|SetSteeringInput (Variables|Default|GetVehicle%20Movement%20Component) ActionValue :!label _label))
  (:Completed
    (goto _label)))

(event Input|EnhancedActionEvents|EnhancedInputActionIA_Vehicle_Throttle
  (params (ActionValue :type Float%20%28double-precision%29) (ElapsedSeconds :type Float%20%28double-precision%29) (TriggeredSeconds :type Float%20%28double-precision%29) (InputAction :type Input%20Action%20Object%20Reference :default "/Game/VehicleConfigurator/Core/Inputs/IA_Vehicle_Throttle.IA_Vehicle_Throttle"))
  (:Triggered
    (Class|ChaosVehicleMovementComponent|SetThrottleInput (Variables|Default|GetVehicle%20Movement%20Component) ActionValue :!label _label))
  (:Completed
    (goto _label)))

(event Input|EnhancedActionEvents|EnhancedInputActionIA_Vehicle_Brake
  (params (ActionValue :type Float%20%28double-precision%29) (ElapsedSeconds :type Float%20%28double-precision%29) (TriggeredSeconds :type Float%20%28double-precision%29) (InputAction :type Input%20Action%20Object%20Reference :default "/Game/VehicleConfigurator/Core/Inputs/IA_Vehicle_Brake.IA_Vehicle_Brake"))
  (:Triggered
    (Class|ChaosVehicleMovementComponent|SetBrakeInput (Variables|Default|GetVehicle%20Movement%20Component) ActionValue :!label _label))
  (:Completed
    (goto _label)))

(event EventBeginPlay
  (bind _aswheeled_vehicle_pawn (Utilities|Casting|CastToWheeledVehiclePawn (Components|GetOwner)))
  (Variables|Default|SetVehicle%20Movement%20Component (Variables|/Script/ChaosVehicles.WheeledVehiclePawn|GetVehicleMovementComponent _aswheeled_vehicle_pawn)))

(event EventTick
  (params (DeltaSeconds :type Float%20%28single-precision%29)))